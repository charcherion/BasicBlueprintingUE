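; Spotlight Blueprint that toggles brightness and random color through the MPC_Sequencer Material Parameter Collection, apparently for Sequencer-driven use.
; MPCLightON and MPCLightOFF read their scalar parameters from the collection and apply them as the SpotLight intensity.
; MPCLightOFF also calls ChangeColor, which picks a random array color, stores it, writes it to the collection's vector parameter and applies it to the light.
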(event `MPC Light ON`
  ; Custom Event grabs Scalar Parameter from set MPC and sets Intencity accordingly (On -> Check MPC)
  (bind _returnvalue (`KismetMaterialLibrary.GetScalarParameterValue` "/Game/1604/MPC_Sequencer.MPC_Sequencer" "Light ON"))
  (`LightComponent.SetIntensity` (`self.SpotLight`) _returnvalue))

(event `MPC Light OFF`
  ; Custom Event grabs Scalar Parameter from set MPC and sets Intencity accordingly (Off -> Check MPC)
  (bind _returnvalue (`KismetMaterialLibrary.GetScalarParameterValue` "/Game/1604/MPC_Sequencer.MPC_Sequencer" "Light OFF"))
  (`LightComponent.SetIntensity` (`self.SpotLight`) _returnvalue)
  ; Call Function Change Color (custom event) on MPC
  ; Light OFF
  (`self.Change Color`))

(event `Change Color`
  ; Custom Event that grabs colors from an array, sets vector parameter value inside of the MPC and sets light color accordingly (+stores the color in case of future use)
  (bind _output_get (set `self.Stored Color` (`|GetArrayItem` (`self.Light Color`) (`KismetMathLibrary.RandomIntegerInRange` 0 5))))
  (`KismetMaterialLibrary.SetVectorParameterValue` "/Game/1604/MPC_Sequencer.MPC_Sequencer" "Random Color" _output_get)
  (`LightComponent.SetLightColor` (`self.SpotLight`) (`self.Stored Color`) true))

(fn `UserConstructionScript`)