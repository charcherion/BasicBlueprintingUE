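; BP_SequenceColor is a light Blueprint that exposes custom events for switching its point light between preset colors.
; Yellow, Green and Purple each set the PointLight to a shared intensity variable and apply their fixed color.
; RandomColor picks one of the three colors at random and applies it, leaving intensity unchanged.
; Nothing in this file calls the events, and the ColorArray variable is unused.
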(event `Yellow`
  (bind _pointlight (`self.PointLight`))
  ;[0.15 0.1475 0.02549 0.5] Custom event calls certain intencity and sets fixed color (yellow)
  (`LightComponent.SetIntensity` _pointlight (`self.Light Intencity`))
  (`LightComponent.SetLightColor` _pointlight (`self.YellowColor`) true))

(event `Green`
  (bind _pointlight (`self.PointLight`))
  ;[0.02549 0.15 0.02798 0.5] Custom event calls certain intencity and sets fixed color (green)
  (`LightComponent.SetIntensity` _pointlight (`self.Light Intencity`))
  (`LightComponent.SetLightColor` _pointlight (`self.GreenColor`) true))

(event `Random Color`
  ; custom event sets color
  (`LightComponent.SetLightColor` (`self.PointLight`) (`|GetArrayItem` (`|MakeArray` (`self.YellowColor`) (`self.GreenColor`) (`self.PurpleColor`)) (`KismetMathLibrary.RandomIntegerInRange` 0 2)) true))

(event `Purple`
  (bind _pointlight (`self.PointLight`))
  ;[0.1477 0.03184 0.15 0.5] Custom event calls certain intencity and sets fixed color (purp)
  (`LightComponent.SetIntensity` _pointlight (`self.Light Intencity`))
  (`LightComponent.SetLightColor` _pointlight (`self.PurpleColor`) true))

(fn `UserConstructionScript`)